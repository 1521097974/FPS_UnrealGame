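; Enemy AI character for an FPS that hurts the player on contact and can be killed by projectiles.
; Overlapping the player character applies damage and adds a bleeding-effect widget to the viewport.
; Projectile hits on the damage capsule drain health; death awards score through the player's attribute component, then destroys the actor after a delay.
; Any hit on that capsule also pushes the character backward with a swept local offset.
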(event OnComponentHit(Capsule_Damage)
  (params (HitComponent :type Primitive%20Component%20Object%20Reference) (OtherActor :type Actor%20Object%20Reference) (OtherComp :type Primitive%20Component%20Object%20Reference) (NormalImpulse :type Vector :default "0, 0, 0") (Hit :type Hit%20Result%20Structure%20%28by%20ref%29))
  ;[1 1 1] 子弹伤害
  (Utilities|FlowControl|Sequence
    (:then_0
      (Utilities|Casting|CastToBP_FPSProjectile OtherActor)
      (Variables|Default|SetHealth (- (Variables|Default|GetHealth) 0.1))
      (if (< (Variables|Default|GetHealth) 0.0)
        (if (not (Variables|Default|GetDead?))
          (Variables|Default|SetDead? true)
          (Class|FPSAttributeComponent|AddScore (Actor|GetComponentbyClass (Game|GetPlayerCharacter 0) "/Script/Tencent_FPS.FPS_AttributeComponent"))
          (Utilities|FlowControl|Delay 2.0)
          (Actor|DestroyActor))))
    (:then_2
      (Transformation|AddActorLocalOffset "-50.000000,0.000000, 0" true false))))

(event EventBeginPlay)

(event Collision|EventActorBeginOverlap
  (params (OtherActor :type Actor%20Object%20Reference))
  ;[1 1 1] 受到伤害
  (bind _asbp_fpscharacter (Utilities|Casting|CastToBP_FPSCharacter OtherActor))
  (Class|FPSCharacter|Damage _asbp_fpscharacter 0.2)
  ;;[1 1 1] 流血效果
  (bind _returnvalue (UserInterface|CreateWidget "/Game/Blueprints/UI/BP_FPSDamegeUI.BP_FPSDamegeUI_C"))
  (UserInterface|Viewport|AddtoViewport _returnvalue 0))

(fn ConstructionScript)